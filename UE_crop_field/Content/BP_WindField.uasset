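; BP_WindField is an actor that publishes global wind settings to materials through the MPC_WindField material parameter collection.
; Every tick it writes game time as WindTime along with mean speed, gust strength, turbulence strength and wind direction from its own variables.
; It computes no wind itself, leaving any gust or turbulence evaluation to whatever reads the collection.
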(event `self.ReceiveTick`
  (params (DeltaSeconds :type "Float (single-precision)"))
  (`KismetMaterialLibrary.SetScalarParameterValue` "/Game/MPC_WindField.MPC_WindField" "WindTime" (`KismetSystemLibrary.GetGameTimeInSeconds`))
  (`KismetMaterialLibrary.SetScalarParameterValue` "/Game/MPC_WindField.MPC_WindField" "WindSpeed" (`self.MeanWindSpeed`))
  (`KismetMaterialLibrary.SetScalarParameterValue` "/Game/MPC_WindField.MPC_WindField" "GustStrength" (`self.GustStrength`))
  (`KismetMaterialLibrary.SetScalarParameterValue` "/Game/MPC_WindField.MPC_WindField" "TurbulenceStrength" (`self.TurbulenceStrength`))
  (`KismetMaterialLibrary.SetVectorParameterValue` "/Game/MPC_WindField.MPC_WindField" "WindDirection" (`KismetMathLibrary.Conv_VectorToLinearColor` (`self.WindDirection`))))

(fn `UserConstructionScript`)